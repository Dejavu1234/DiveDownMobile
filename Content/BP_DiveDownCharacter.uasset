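; BP_DiveDownCharacter is a character Blueprint that handles virtual joystick movement and look, and records touch position.
; Move axes add forced movement along directions built from control pitch only, with yaw and roll zeroed.
; Look axes add controller yaw and pitch, scaled by base rates and delta time.
; Finger1 presses and any touch move store Touch1's screen position in CurrentTouch, which nothing here reads.
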(event `InputAxis|MoveForward`
  (params (AxisValue :type "Float (single-precision)"))
  ;[1 1 1] Virtual Joysticks
  (`self.AddMovementInput` (`KismetMathLibrary.GetForwardVector` (`KismetMathLibrary.MakeRotator` 0.0 (.pitch (`self.GetControlRotation`)))) AxisValue true))

(event `InputAxis|MoveRight`
  (params (AxisValue :type "Float (single-precision)"))
  ;[1 1 1] Virtual Joysticks
  (`self.AddMovementInput` (`KismetMathLibrary.GetRightVector` (`KismetMathLibrary.MakeRotator` 0.0 (.pitch (`self.GetControlRotation`)))) AxisValue true))

(event `InputAxis|TurnRaTE`
  (params (AxisValue :type "Float (single-precision)"))
  ;[1 1 1] Virtual Joysticks
  (`self.AddControllerYawInput` (* AxisValue (`GameplayStatics.GetWorldDeltaSeconds`) (`self.BaseTurnRate`))))

(event `InputAxis|LookUpRate`
  (params (AxisValue :type "Float (single-precision)"))
  ;[1 1 1] Virtual Joysticks
  (`self.AddControllerPitchInput` (* AxisValue (`GameplayStatics.GetWorldDeltaSeconds`) (`self.BaseLookUpRate`))))

(event `self.ReceiveBeginPlay`)

(event `self.ReceiveTick`
  (params (DeltaSeconds :type "Float (single-precision)"))
  ;[1 1 1] Recording whole screen mouse/finger Position
)

(event `InputAction|Finger1`
  (params (Key :type "Key Structure"))
  (bind (_locationx _locationy) (`PlayerController.GetInputTouchState` (`GameplayStatics.GetPlayerController` 0) "Touch1"))
  ;[1 1 1] Recording whole screen mouse/finger Position
  (:`Pressed`
    (set `self.CurrentTouch` (`KismetMathLibrary.MakeVector2D` _locationx _locationy) :!label _label)))

(event `InputTouch`
  (params (Location :type "Vector Structure") (FingerIndex :type "ETouchIndex Enum"))
  ;[1 1 1] Recording whole screen mouse/finger Position
  (:`Moved`
    (goto _label)))

(fn `UserConstructionScript`)